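; Player character for Kim with move, look and jump input, plus a turret building mode.
; Turret selection async-loads a data asset from TurretMap and spawns a BP_Turret_MachineGun preview.
; Each tick, a camera line trace moves the preview, and a box trace sets placement validity and green/red hologram material.
; Shooting places valid turrets and spawns another preview; deselect destroys it, while snapping logic is disconnected.
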(event `self.ReceiveBeginPlay`
  ;[1 1 1] Bind IMC to main character
  (bind _asbp_kim_player_controller (cast `/Game/Core/BP_KimPlayerController` (`self.GetController`)))
  (`EnhancedInputSubsystemInterface.AddMappingContext` (pcsubsystem `EnhancedInputLocalPlayerSubsystem` _asbp_kim_player_controller) "/Game/Core/Inputs/IMC_KimDefault.IMC_KimDefault" 0 (struct)))

(event `EnhancedInput|/Game/Core/Inputs/IA_KimLook`
  (params (ActionValue :type "Vector2D Structure") (ElapsedSeconds :type "Float (double-precision)") (TriggeredSeconds :type "Float (double-precision)") (InputAction :type "InputAction Object Reference" :default "/Game/Core/Inputs/IA_KimLook.IA_KimLook"))
  ;[1 1 1] Movement and Look inputs
  (:`Triggered`
    (`self.AddControllerYawInput` ActionValue_X)
    (`self.AddControllerPitchInput` ActionValue_Y)))

(event `EnhancedInput|/Game/Core/Inputs/IA_KimMove`
  (params (ActionValue :type "Vector2D Structure") (ElapsedSeconds :type "Float (double-precision)") (TriggeredSeconds :type "Float (double-precision)") (InputAction :type "InputAction Object Reference" :default "/Game/Core/Inputs/IA_KimMove.IA_KimMove"))
  ;[1 1 1] Movement and Look inputs
  (:`Triggered`
    (`self.AddMovementInput` (`self.GetActorRightVector`) ActionValue_X)
    (`self.AddMovementInput` (`self.GetActorForwardVector`) ActionValue_Y)))

(event `EnhancedInput|/Game/Core/Inputs/IA_Jump`
  (params (ActionValue :type Boolean) (ElapsedSeconds :type "Float (double-precision)") (TriggeredSeconds :type "Float (double-precision)") (InputAction :type "InputAction Object Reference" :default "/Game/Core/Inputs/IA_Jump.IA_Jump"))
  ;[1 1 1] Input jump
  (:`Triggered`
    (`self.Jump`))
  (:`Completed`
    (`self.StopJumping`)))

(event `EnhancedInput|/Game/Core/Inputs/IA_Shoot_Place`
  (params (ActionValue :type Boolean) (ElapsedSeconds :type "Float (double-precision)") (TriggeredSeconds :type "Float (double-precision)") (InputAction :type "InputAction Object Reference" :default "/Game/Core/Inputs/IA_Shoot_Place.IA_Shoot_Place"))
  (:`Triggered`
    (if (`self.BuildingModeActive`)
      (if (`self.IsValidPlacement`)
        (`self.PlaceTurret`)
        (set `self.MachineGun` null)
        (`self.SpawnNewTurret` (`/Game/Core/Data_Assets/DA_Blueprints.Turret` (stale `EnhancedInput|/Game/Core/Inputs/IA_TurretSelect` _asda_blueprints)) (stale `EnhancedInput|/Game/Core/Inputs/IA_TurretSelect` _output_get) :!label _label)))))

(event `EnhancedInput|/Game/Core/Inputs/IA_TurretSelect`
  (params (ActionValue :type "Float (double-precision)") (ElapsedSeconds :type "Float (double-precision)") (TriggeredSeconds :type "Float (double-precision)") (InputAction :type "InputAction Object Reference" :default "/Game/Core/Inputs/IA_TurretSelect.IA_TurretSelect"))
  (bind (_value _returnvalue) (`BlueprintMapLibrary.Map_Find` (`self.TurretMap`) (`KismetMathLibrary.Round` ActionValue)))
  (:`Triggered`
    (set `self.BuildingModeActive` _returnvalue)
    (bind _output_get (set `self.DataAssetUsed` _value))
    (if (`KismetSystemLibrary.IsValidSoftObjectReference` _output_get)
      (bind _object (`|LoadAsset` _output_get)
        (:`then`
          (bind _asda_blueprints (cast `/Game/Core/Data_Assets/DA_Blueprints` _object))
          (goto _label)))
      (else
        (`self.K2_DestroyActor`)))))

(event `self.ReceiveTick`
  (params (DeltaSeconds :type "Float (single-precision)"))
  (`self.UpdateTurretLocation`))

(event `EnhancedInput|/Game/Core/Inputs/IA_Vacuum_Deselect`
  (params (ActionValue :type Boolean) (ElapsedSeconds :type "Float (double-precision)") (TriggeredSeconds :type "Float (double-precision)") (InputAction :type "InputAction Object Reference" :default "/Game/Core/Inputs/IA_Vacuum_Deselect.IA_Vacuum_Deselect"))
  (:`Triggered`
    (bind _machinegun (`self.MachineGun`)
      (:`then`
        (`self.K2_DestroyActor` _machinegun))
      (:`else`))))

(fn `CanBePlaced`
  (bind _machinegun (`self.MachineGun`))
  (bind _returnvalue (`self.GetComponentByClass` _machinegun "/Script/Engine.StaticMeshComponent"))
  (bind _origin (`KismetSystemLibrary.GetComponentBounds` _returnvalue))
  (bind (_outhit _returnvalue_2) (`KismetSystemLibrary.BoxTraceSingle` :`Start` _origin :`End` _origin :`HalfSize` (* (- (`.Max` (`StaticMeshComponent.GetLocalBounds` _returnvalue)) (`KismetMathLibrary.InverseTransformLocation` (`self.GetTransform` _machinegun) _origin)) 0.5) :`Orientation` (`self.K2_GetActorRotation` (`self.MachineGun`)) :`TraceChannel` "TraceTypeQuery1" :`DrawDebugType` "ForOneFrame"))
  (set `self.IsValidPlacement` (not _returnvalue_2))
  (`PrimitiveComponent.SetMaterial` (`/Game/Blueprints/Turrets/BP_Turret_MachineGun.StaticMesh` (`self.MachineGun`)) 0 (select `bool` (`self.IsValidPlacement`) :`false` "/Game/Core/Materials/M_Hologram_Red.M_Hologram_Red" :`true` "/Game/Core/Materials/M_Hologram_Green.M_Hologram_Green" :!type "MaterialInterface Object Reference")))

(fn `PlaceTurret`
  (bind _returnvalue (`self.GetComponentByClass` (`self.MachineGun`) "/Script/Engine.StaticMeshComponent"))
  (`PrimitiveComponent.SetMaterial` _returnvalue 0 "/Engine/BasicShapes/BasicShapeMaterial.BasicShapeMaterial")
  (`PrimitiveComponent.SetCollisionEnabled` _returnvalue "QueryAndPhysics"))

(fn `SpawnNewTurret`
  (params (InputPin :type "Actor Class Reference") (NewParam :type "/Game/Core/Data_Assets/DA_Blueprints Soft Object Reference"))
  (bind _machinegun (`self.MachineGun`)
    (:`then`
      (`self.K2_DestroyActor` _machinegun))
    (:`else`
      _))
  (bind _outhit (`self.LineTraceByChannelFRWD`))
  (bind _returnvalue (`|SpawnActorFromClass` "/Game/Blueprints/Turrets/BP_Turret_MachineGun.BP_Turret_MachineGun_C" (`KismetMathLibrary.MakeTransform` (`.ImpactPoint` (`GameplayStatics.BreakHitResult` _outhit))) "Undefined" "MultiplyWithRoot" null NewParam (cast `Pawn` (`self.GetOwner`) :!pure true)))
  (set `self.MachineGun` _returnvalue))

(fn `UpdateTurretLocation`
  (locals (`L-ImpactPoint` :type "Vector Structure") (`L-HitActor` :type "/Game/Blueprints/Turrets/BP_Turret_MachineGun Object Reference") (`L-SnapPoint` :type "Transform Structure"))
  (`self.MachineGun`
    (:`then`
      (`|ExecutionSequence`
        (:`then_0`
          (bind _outhit (`self.LineTraceByChannelFRWD`))
          (`self.K2_SetActorLocation` (`self.MachineGun`) (`.ImpactPoint` (`GameplayStatics.BreakHitResult` _outhit)) false true))
        (:`then_1`
          (`self.CanBePlaced`))))
    (:`else`)))

(fn `UserConstructionScript`)