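; Machine gun turret actor that takes its mesh and filtered snap points from a DA_Blueprints data asset.
; BeginPlay loads that asset synchronously, or destroys the actor if the reference is invalid; SaveDataAsset writes mesh and points back.
; Without an instigator, the construction script syncs SnapPoints into SnapPointFilter, keeping filters by index and trimming surplus entries from the front.
; GetClosestTransform searches in local space for the snap point nearest an impact, returning world location and rotation.
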(event `self.ReceiveBeginPlay`
  (if (`KismetSystemLibrary.IsValidSoftObjectReference` (`self.DataAssetUsed`))
    (`self.LoadDataAsset`)
    (else
      (`self.K2_DestroyActor`))))

(fn `GetClosestTransform`
  (params (ImpactPoint :type "Vector Structure"))
  (returns (ReturnValue :type "Transform Structure"))
  (locals (`L-TestingLocation` :type "Vector Structure" :default (0.0 0.0 0.0)) (`L-Distance` :type "Float (double-precision)" :default 1000000.0) (ReturnTrasform :type "Transform Structure"))
  (bind _returnvalue (`self.GetTransform`))
  (bind (_returntrasform_location _returntrasform_rotation _returntrasform_scale) (`KismetMathLibrary.BreakTransform` (`local.ReturnTrasform`)))
  (set `local.L-TestingLocation` (`KismetMathLibrary.InverseTransformLocation` (`self.GetTransform`) ImpactPoint))
  (for _array_element (`self.SnapPointFilter`)
    (bind _returnvalue_2 (`KismetMathLibrary.Vector_Distance` (.location (break `/Game/Blueprints/ST_SnapPoint` _array_element)) (`local.L-TestingLocation`)))
    (if (< _returnvalue_2 (`local.L-Distance`))
      (set `local.L-Distance` _returnvalue_2)
      (set `local.ReturnTrasform` (break `/Game/Blueprints/ST_SnapPoint` _array_element))))
  (return (`KismetMathLibrary.MakeTransform` (`KismetMathLibrary.TransformLocation` _returnvalue _returntrasform_location) (`KismetMathLibrary.TransformRotation` _returnvalue _returntrasform_rotation) _returntrasform_scale)))

(fn `LoadDataAsset`
  (bind _dataassetused (`self.DataAssetUsed`))
  (if (`KismetSystemLibrary.IsValidSoftObjectReference` _dataassetused)
    (bind _returnvalue (`KismetSystemLibrary.LoadAsset_Blocking` _dataassetused))
    (bind _asda_blueprints (cast `/Game/Core/Data_Assets/DA_Blueprints` _returnvalue))
    (set `self.SnapPointFilter` (`/Game/Core/Data_Assets/DA_Blueprints.SnapPoints` _asda_blueprints))
    (`KismetArrayLibrary.Array_Clear` (`self.SnapPoints`))
    (for (_array_element _array_index) (`self.SnapPointFilter`)
      (`KismetArrayLibrary.Array_Set` (`self.SnapPoints`) _array_index (`.SnapPoint_3_1C49ABF64D781F2C13B220887FE30640` (break `/Game/Blueprints/ST_SnapPoint` _array_element)) true))
    (bind _returnvalue_2 (`KismetSystemLibrary.LoadAsset_Blocking` (`/Game/Core/Data_Assets/DA_Blueprints.TurretMesh` _asda_blueprints)))
    (bind _asstatic_mesh (cast `StaticMesh` _returnvalue_2))
    (`StaticMeshComponent.SetStaticMesh` (`self.StaticMesh`) _asstatic_mesh)))

(fn `SaveDataAsset`
  (bind _dataassetused (`self.DataAssetUsed`))
  (if (`KismetSystemLibrary.IsValidSoftObjectReference` _dataassetused)
    (bind _returnvalue (`KismetSystemLibrary.LoadAsset_Blocking` _dataassetused))
    (bind _asda_blueprints (cast `/Game/Core/Data_Assets/DA_Blueprints` _returnvalue))
    (set `/Game/Core/Data_Assets/DA_Blueprints.SnapPoints` (`self.SnapPointFilter`) _asda_blueprints)
    (set `/Game/Core/Data_Assets/DA_Blueprints.TurretMesh` (`|ConvertAsset` (`StaticMeshComponent.StaticMesh` (`self.StaticMesh`))) _asda_blueprints)))

(fn `UserConstructionScript`
  (bind _snappointfilter (`self.SnapPointFilter`))
  (`/Engine/EditorBlueprintResources/StandardMacros.IsValid` (`self.GetInstigator`)
    (:`Is Not Valid`
      (for (_array_element _array_index) (`self.SnapPoints`)
        (bind (_output_snappoint _output_filter) (break `/Game/Blueprints/ST_SnapPoint` (`|GetArrayItem` _snappointfilter _array_index)))
        (`KismetArrayLibrary.Array_Set` _snappointfilter _array_index (make `/Game/Blueprints/ST_SnapPoint` _array_element _output_filter) true))
      (while (< (`KismetArrayLibrary.Array_Length` (`self.SnapPoints`)) (`KismetArrayLibrary.Array_Length` (`self.SnapPointFilter`)))
        (`KismetArrayLibrary.Array_Remove` (`self.SnapPointFilter`))))))